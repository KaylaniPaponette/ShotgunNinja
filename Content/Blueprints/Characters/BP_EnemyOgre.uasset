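; BP_EnemyOgre is an ogre enemy character that takes damage and is destroyed when its health runs out.
; AnyDamage forwards damage to TakeDamage, which applies it through the ACHealthComp component and destroys the actor if dead, otherwise printing remaining health.
; An unconnected chain of test calls exercising the health component's damage and heal functions remains in the event graph.
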(event EventBeginPlay)

(event Collision|EventActorBeginOverlap
  (params (OtherActor :type Actor%20Object%20Reference)))

(event EventTick
  (params (DeltaSeconds :type Float%20%28single-precision%29)))

(event Game|Damage|EventAnyDamage
  (params (Damage :type Float%20%28single-precision%29) (DamageType :type Damage%20Type%20Object%20Reference) (InstigatedBy :type Controller%20Object%20Reference) (DamageCauser :type Actor%20Object%20Reference))
  (CallFunction|TakeDamage Damage))

(fn ConstructionScript)

(fn TakeDamage
  (params (DamageAmount :type Float%20%28double-precision%29))
  (bind _ac_healthcomp (Variables|Default|GetAC_HealthComp))
  (Default|Damage _ac_healthcomp DamageAmount)
  (if (Default|IsDead _ac_healthcomp)
    (Actor|DestroyActor)
    (else
      (Development|PrintString (Utilities|String|ToString(Float) (Default|GetHealth _ac_healthcomp))))))