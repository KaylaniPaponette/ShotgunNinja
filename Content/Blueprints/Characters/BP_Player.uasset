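; Player character that handles movement, jumping, a cooldown dash, shotgun combat and pausing.
; BeginPlay spawns and attaches BP_Shotgun before creating the in-game menu; firing casts to it with a DoOnce/Delay rate limit, while reload uses BPIGun.
; Dash chains a small upward launch into a launch along the last movement input.
; Damage feeds ACHealthComp and death opens the main menu, with a debug self-damage key and leftover health-bar update experiments.
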(event Custom|UpdateHealth
  ;[0.15 0.15 0.15 0.5] 3rd method of health bar updating
  (Default|CallOnDamaged))

(event Game|Damage|EventAnyDamage
  (params (Damage :type Float%20%28single-precision%29) (DamageType :type Damage%20Type%20Object%20Reference) (InstigatedBy :type Controller%20Object%20Reference) (DamageCauser :type Actor%20Object%20Reference))
  ;[0.15 0.15 0.15 0.5] Take Damage
  (CallFunction|TakeDamage Damage))

(event Collision|EventActorBeginOverlap
  (params (OtherActor :type Actor%20Object%20Reference)))

(event EventTick
  (params (DeltaSeconds :type Float%20%28single-precision%29)))

(event EventBeginPlay
  (bind _returnvalue (Game|GetPlayerController 0))
  (Utilities|FlowControl|Sequence
    (:then_0
      ;[0.15 0.15 0.15 0.5] Spawn SG (must occur before UI is created or the GetAmmoText Function will fail
      (bind _returnvalue_2 (Game|SpawnActorfromClass "/Game/Blueprints/Weapons/BP_Shotgun.BP_Shotgun_C" (Math|Transform|MakeTransform "0, 0, 0" "0, 0, 0" "1.000000,1.000000,1.000000") "Undefined" "MultiplyWithRoot" 0 0))
      (bind _output_get (Variables|Components|SetSGRef _returnvalue_2))
      (Transformation|AttachComponentToComponent _output_get (Variables|Default|GetSGSpawnPoint) "None" "SnapToTarget" "SnapToTarget" "SnapToTarget" true))
    (:then_1
      ;[0.15 0.15 0.15 0.5] Adds InGameMenu to Viewport and gets health at the start of the gaqme
      (bind _returnvalue_3 (UserInterface|CreateWidget "/Game/Blueprints/GUI/WBP_InGameMenu.WBP_InGameMenu_C"))
      (UserInterface|Viewport|AddtoViewport _returnvalue_3 0))
    (:then_2
      (Input|SetInputModeGameOnly _returnvalue false)
      (Variables|/Script/Engine.PlayerController|SetbShowMouseCursor _returnvalue false))))

(event Input|ActionEvents|InputActionJump
  (params (Key :type Key%20Structure :default "None"))
  ;[0.15 0.15 0.15 0.5] Action Map - Jumping
  (:Pressed
    (Character|Jump)))

(event Input|ActionEvents|InputActionReload
  (params (Key :type Key%20Structure :default "None"))
  ;[0.15 0.15 0.15 0.5] Reload
  (:Pressed
    (bind _asbpigun (Utilities|Casting|CastToBPIGun (Variables|Components|GetSGRef)))
    (Default|Reload _asbpigun)))

(event Input|ActionEvents|InputActionDash
  (params (Key :type Key%20Structure :default "None"))
  ;[0.15 0.15 0.15 0.5] Dash
  (:Pressed
    (Utilities|FlowControl|DoOnce false :!label _label
      (:Completed
        (Character|LaunchCharacter (* (Math|Vector|GetUpVector "0, 0, 0") "0.000000,0.000000,150.000000") false false)
        (Utilities|FlowControl|Delay 0.001)
        (Character|LaunchCharacter (* (Math|Vector|Normalize (Pawn|Components|PawnMovement|GetLastInputVector (Variables|Character|GetCharacterMovement))) (Math|Vector|MakeVector 1.5e+03 1.5e+03 0.0)) false false)
        (Utilities|FlowControl|Delay 0.5)
        (goto _label Reset)))))

(event Input|ActionEvents|InputActionPause
  (params (Key :type Key%20Structure :default "None"))
  (bind _returnvalue (Game|GetPlayerController 0))
  ;[0.15 0.15 0.15 0.5] Pause
  (:Pressed
    (bind _returnvalue_2 (UserInterface|CreateWidget "/Game/Blueprints/GUI/WBP_PauseMenu.WBP_PauseMenu_C"))
    (UserInterface|Viewport|AddtoViewport _returnvalue_2 0)
    (Variables|/Script/Engine.PlayerController|SetbShowMouseCursor _returnvalue true)
    (Input|SetInputModeUIOnly _returnvalue 0 "DoNotLock" false)
    (Game|SetGamePaused true)))

(event Input|AxisEvents|InputAxisTurn
  (params (AxisValue :type Float%20%28single-precision%29))
  ;[0.15 0.15 0.15 0.5] Camera
  (Pawn|Input|AddControllerYawInput AxisValue))

(event Input|AxisEvents|InputAxisLookUp
  (params (AxisValue :type Float%20%28single-precision%29))
  ;[0.15 0.15 0.15 0.5] Camera
  (Pawn|Input|AddControllerPitchInput AxisValue))

(event Input|AxisEvents|InputAxisMove_Forward
  (params (AxisValue :type Float%20%28single-precision%29))
  ;[0.15 0.15 0.15 0.5] Movement
  (Pawn|Input|AddMovementInput (Math|Vector|GetForwardVector (Variables|Collision|GetCapsuleComponent)) AxisValue false))

(event Input|AxisEvents|InputAxisStrafe
  (params (AxisValue :type Float%20%28single-precision%29))
  ;[0.15 0.15 0.15 0.5] Movement
  (Pawn|Input|AddMovementInput (Math|Vector|GetRightVector (Variables|Collision|GetCapsuleComponent)) AxisValue false))

(event Input|AxisEvents|InputAxisShoot
  (params (AxisValue :type Float%20%28single-precision%29))
  ;[0.15 0.15 0.15 0.5] Fire
  (if (>= AxisValue 0.1)
    (Utilities|FlowControl|DoOnce false :!label _label
      (:Completed
        (bind _asbp_shotgun (Utilities|Casting|CastToBP_Shotgun (Variables|Components|GetSGRef)))
        (Default|Shoot _asbp_shotgun)
        (Utilities|FlowControl|Delay 0.8)
        (goto _label Reset)))))

(event Input|KeyboardEvents|1
  (params (Key :type Key%20Structure :default "None"))
  ;[0.15 0.15 0.15 0.5] test health bar - damage when pressing 1
  (:Pressed
    (Game|Damage|ApplyDamage self 1e+01 0 0)))

(fn ConstructionScript)

(fn TakeDamage
  (params (Damage%20Amount :type Float%20%28double-precision%29))
  (bind _ac_healthcomp (Variables|Default|GetAC_HealthComp))
  (Default|Damage _ac_healthcomp Damage%20Amount)
  (if (Default|IsDead _ac_healthcomp)
    (Game|OpenLevel(byObjectReference) "/Game/Maps/MainMenuMap.MainMenuMap")
    (else
      (Development|PrintString (Utilities|String|ToString(Float) (Default|GetHealth _ac_healthcomp))))))