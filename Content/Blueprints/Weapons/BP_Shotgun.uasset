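; BP_Shotgun is a shotgun weapon Blueprint that handles firing and reloading with a simple ammo counter.
; Shoot checks for remaining ammo, decrements it, prints the count and spawns a single actor at the BulletSpawnPoint transform.
; Reload instantly restores CurrentAmmo to MaxAmmo and prints a confirmation, with no reserve pool or delay.
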(event Collision|EventActorBeginOverlap
  (params (OtherActor :type Actor%20Object%20Reference)))

(event EventTick
  (params (DeltaSeconds :type Float%20%28single-precision%29)))

(event EventShoot
  ;[0.15 0.15 0.15 0.5] Shooting
  (if (> (Variables|Default|GetCurrent%20Ammo) 0)
    (Math|Integer|DecrementInt (Variables|Default|GetCurrent%20Ammo)
      (:%20%20
        (Development|PrintString (Utilities|String|ToString(Integer) (Variables|Default|GetCurrent%20Ammo)))
        (Game|SpawnActorfromClass "/Game/Blueprints/Weapons/BP_SGProjectile.BP_SGProjectile_C" (Transformation|GetWorldTransform (Variables|Default|GetBulletSpawnPoint)) "Undefined" "MultiplyWithRoot" 0 0)))))

(event EventReload
  ;[0.15 0.15 0.15 0.5] Reloading
  (Variables|Default|SetCurrent%20Ammo (Variables|Default|GetMax%20Ammo))
  (Development|PrintString "Gun Reloaded"))

(fn ConstructionScript)