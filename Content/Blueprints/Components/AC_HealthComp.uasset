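; Health component that gives its owning actor a health pool with damage, healing, full heal, kill, death check and normalized health queries.
; On BeginPlay, Init applies the configured min and max bounds and starts health at maximum.
; Heal and Damage accept only positive amounts, printing a message otherwise, and route through SetHealth, which clamps to those bounds.
; It broadcasts no events, so death and health changes are only visible by querying it.
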(event EventBeginPlay
  (CallFunction|Init (Variables|Default|GetMinHealth) (Variables|Default|GetMaxHealth)))

(fn Heal
  (params (HealAmount :type Float%20%28double-precision%29))
  (if (> HealAmount 0.0)
    (CallFunction|SetHealth (+ (CallFunction|GetHealth) HealAmount))
    (else
      (Development|PrintString "Heal has to be positive"))))

(fn GetHealth
  (return (Variables|Default|GetHealth)))

(fn SetHealth
  (params (NewHealth :type Float%20%28double-precision%29))
  (bind _output_get (Variables|Default|SetHealth (CallFunction|ClampHealth NewHealth)))
  (return _output_get))

(fn ClampHealth
  (params (Value :type Float%20%28double-precision%29))
  (return (Math|Float|Clamp(Float) Value (Variables|Default|GetMinHealth) (Variables|Default|GetMaxHealth))))

(fn Damage
  (params (Damage%20Amount :type Float%20%28double-precision%29))
  (if (> Damage%20Amount 0.0)
    (CallFunction|SetHealth (- (CallFunction|GetHealth) Damage%20Amount))
    (else
      (Development|PrintString "Damage has to be positive"))))

(fn IsDead
  (return (<= (CallFunction|GetHealth) (Variables|Default|GetMinHealth))))

(fn GetNormalizedHealth
  (return (Math|Float|Clamp(Float) (/ (CallFunction|GetHealth) (Variables|Default|GetMaxHealth)))))

(fn HealFull
  (CallFunction|Heal (Variables|Default|GetMaxHealth)))

(fn Kill
  (CallFunction|Damage (Variables|Default|GetMaxHealth)))

(fn Init
  (params (NewMinHealth :type Float%20%28double-precision%29) (NewMaxHealth :type Float%20%28double-precision%29))
  (Variables|Default|SetMinHealth NewMinHealth)
  (bind _output_get (Variables|Default|SetMaxHealth NewMaxHealth))
  (CallFunction|SetHealth _output_get))