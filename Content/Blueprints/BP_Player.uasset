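; Player character Blueprint that handles first-stage input for looking, moving, strafing, jumping, shooting and reloading.
; On BeginPlay it spawns a BP_Shotgun, stores it in SGRef and snaps it to the SGSpawnPoint component.
; Held Shoot axis input passes through a Delay, pacing and postponing each ShootMessage sent to the shotgun.
; Reload reaches the same weapon through a BPIGun cast.
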(event Collision|EventActorBeginOverlap
  (params (OtherActor :type Actor%20Object%20Reference)))

(event EventTick
  (params (DeltaSeconds :type Float%20%28single-precision%29)))

(event EventBeginPlay
  ;[0.15 0.15 0.15 0.5] Spawn SG
  (bind _returnvalue (Game|SpawnActorfromClass "/Game/Blueprints/BP_Shotgun.BP_Shotgun_C" (Math|Transform|MakeTransform "0, 0, 0" "0, 0, 0" "1.000000,1.000000,1.000000") "Undefined" "MultiplyWithRoot" 0 0))
  (bind _output_get (Variables|Components|SetSGRef _returnvalue))
  (Transformation|AttachComponentToComponent _output_get (Variables|Default|GetSGSpawnPoint) "None" "SnapToTarget" "SnapToTarget" "SnapToTarget" true))

(event Input|ActionEvents|InputActionJump
  (params (Key :type Key%20Structure :default "None"))
  ;[0.15 0.15 0.15 0.5] Action Map - Jumping
  (:Pressed
    (Character|Jump)))

(event Input|ActionEvents|InputActionReload
  (params (Key :type Key%20Structure :default "None"))
  ;[0.15 0.15 0.15 0.5] Reload
  (:Pressed
    (bind _asbpigun (Utilities|Casting|CastToBPIGun (Variables|Components|GetSGRef)))
    (Default|Reload _asbpigun)))

(event Input|AxisEvents|InputAxisTurn
  (params (AxisValue :type Float%20%28single-precision%29))
  ;[0.15 0.15 0.15 0.5] Camera
  (Pawn|Input|AddControllerYawInput AxisValue))

(event Input|AxisEvents|InputAxisLookUp
  (params (AxisValue :type Float%20%28single-precision%29))
  ;[0.15 0.15 0.15 0.5] Camera
  (Pawn|Input|AddControllerPitchInput AxisValue))

(event Input|AxisEvents|InputAxisMove_Forward
  (params (AxisValue :type Float%20%28single-precision%29))
  ;[0.15 0.15 0.15 0.5] Movement
  (Pawn|Input|AddMovementInput (Math|Vector|GetForwardVector (Variables|Collision|GetCapsuleComponent)) AxisValue false))

(event Input|AxisEvents|InputAxisStrafe
  (params (AxisValue :type Float%20%28single-precision%29))
  ;[0.15 0.15 0.15 0.5] Movement
  (Pawn|Input|AddMovementInput (Math|Vector|GetRightVector (Variables|Collision|GetCapsuleComponent)) AxisValue false))

(event Input|AxisEvents|InputAxisShoot
  (params (AxisValue :type Float%20%28single-precision%29))
  ;[0.15 0.15 0.15 0.5] Fire
  (if (>= AxisValue 0.1)
    (Utilities|FlowControl|Delay 0.7)
    (bind _asbp_shotgun (Utilities|Casting|CastToBP_Shotgun (Variables|Components|GetSGRef)))
    (Class|BPIGun|Shoot(Message) _asbp_shotgun)))

(fn ConstructionScript)