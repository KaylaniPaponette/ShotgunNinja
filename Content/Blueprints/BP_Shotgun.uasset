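; BP_Shotgun is a shotgun weapon Blueprint that fires projectiles from a limited ammo count.
; Shoot decrements CurrentAmmo when any remains and spawns a single Projectile actor at the BulletSpawnPoint transform.
; Reload instantly restores CurrentAmmo to MaxAmmo, and both events print debug messages to report the result.
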(event EventBeginPlay)

(event Collision|EventActorBeginOverlap
  (params (OtherActor :type Actor%20Object%20Reference)))

(event EventTick
  (params (DeltaSeconds :type Float%20%28single-precision%29)))

(event EventShoot
  (if (> (Variables|Default|GetCurrent%20Ammo) 0)
    (Math|Integer|DecrementInt (Variables|Default|GetCurrent%20Ammo)
      (:%20%20
        (Development|PrintString (Utilities|String|ToString(Integer) (Variables|Default|GetCurrent%20Ammo)))
        (Game|SpawnActorfromClass "/Game/Blueprints/Projectile.Projectile_C" (Transformation|GetWorldTransform (Variables|Default|GetBulletSpawnPoint)) "Undefined" "MultiplyWithRoot" 0 0)))))

(event EventReload
  (Variables|Default|SetCurrent%20Ammo (Variables|Default|GetMax%20Ammo))
  (Development|PrintString "Gun Reloaded"))

(fn ConstructionScript)